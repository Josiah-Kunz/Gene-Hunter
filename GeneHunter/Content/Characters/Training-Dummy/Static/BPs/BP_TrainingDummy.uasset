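; BP_TrainingDummy is a training dummy character Blueprint with a health bar and cursor mouseover detection.
; On BeginPlay it casts the HealthBarWidget's widget to WB_HealthBar and passes in its CombatStats, printing an error if the cast fails.
; It also hands MouseoverCollider to MouseoverTrigger as the collision component.
; The collider's begin-cursor-over event only prints a debug "Hello".
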(event OnBeginCursorOver(MouseoverCollider)
  (params (TouchedComponent :type Primitive%20Component%20Object%20Reference))
  (Development|PrintString "Hello"))

(event EventBeginPlay
  (CallFunction|InitializeHealthBar)
  (CallFunction|InitializeMouseover))

(event Collision|EventActorBeginOverlap
  (params (OtherActor :type Actor%20Object%20Reference)))

(event EventTick
  (params (DeltaSeconds :type Float%20%28single-precision%29)))

(fn ConstructionScript)

(fn InitializeHealthBar
  (bind _aswb_health_bar (Utilities|Casting|CastToWB_HealthBar (UserInterface|GetWidget (Variables|Default|GetHealth%20Bar%20Widget)))
    (:then
      (Class|HealthBarWidget|SetCombatStats _aswb_health_bar (Variables|Default|GetCombatStats)))
    (:CastFailed
      (Development|PrintString "Uh-oh....cast failed in bp-topdown-char's Initialize Health Bar!"))))

(fn InitializeMouseover
  (Class|MouseoverTrigger|SetCollisionComponent (Variables|Default|GetMouseoverTrigger) (Variables|Default|GetMouseover%20Collider)))