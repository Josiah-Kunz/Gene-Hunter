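; Training dummy Blueprint that patrols along a looping, curve-driven path around its starting location.
; BeginPlay stores the origin, and Tick calls Patrol to sample a vector curve at normalized time over the period, resetting the timer after each cycle.
; Each curve axis blends between that axis's min/max range through LerpRange, and the resulting offset from the origin is applied as a swept move.
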(event EventBeginPlay
  (|CallParentFunction)
  (Variables|Default|SetOG%20Location (Transformation|GetActorLocation)))

(event Collision|EventActorBeginOverlap
  (params (OtherActor :type Actor%20Object%20Reference))
  (|CallParentFunction OtherActor) ; This node is disabled and will not be called.\nDrag off pins to build functionality.
)

(event EventTick
  (params (DeltaSeconds :type Float%20%28single-precision%29))
  (|CallParentFunction DeltaSeconds)
  (CallFunction|Patrol DeltaSeconds))

(fn ConstructionScript
  (|CallParentFunction))

(fn Patrol
  (params (DeltaSeconds :type Float%20%28double-precision%29))
  ;[1 1 1] Lerp based on curve
  (bind _result (CallFunction|LerpRange (Variables|Patrol|GetX%20Range) (.X (Math|Vector|BreakVector (Math|Curves|GetVectorValue (Variables|Patrol|GetPatrol%20Curve) (/ (Variables|Default|Gett) (Variables|Patrol|GetPeriod)))))))
  (bind _result_2 (CallFunction|LerpRange (Variables|Patrol|GetY%20Range) (.Y (Math|Vector|BreakVector (Math|Curves|GetVectorValue (Variables|Patrol|GetPatrol%20Curve) (/ (Variables|Default|Gett) (Variables|Patrol|GetPeriod)))))))
  (bind _result_3 (CallFunction|LerpRange (Variables|Patrol|GetZ%20Range) (.Z (Math|Vector|BreakVector (Math|Curves|GetVectorValue (Variables|Patrol|GetPatrol%20Curve) (/ (Variables|Default|Gett) (Variables|Patrol|GetPeriod)))))))
  ;[1 1 1] Move the actor
  (Transformation|SetActorLocation (+ (Math|Vector|MakeVector _result _result_2 _result_3) (Variables|Default|GetOG%20Location)) true false)
  ;[1 1 1] Increment Time
  (bind _output_get (Variables|Default|Sett (+ DeltaSeconds (Variables|Default|Gett))))
  (if (> _output_get (Variables|Patrol|GetPeriod))
    (Variables|Default|Sett 0.0)))

(fn LerpRange
  (params (Range :type Vector%202D%20Structure) (Fraction :type Float%20%28double-precision%29))
  (bind (_x _y) (Math|Vector2D|BreakVector2D Range))
  (return (Math|Float|Lerp _x _y Fraction)))