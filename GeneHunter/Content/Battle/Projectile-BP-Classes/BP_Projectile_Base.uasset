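; Base Blueprint for battle projectiles that detects contact with actors carrying a CombatStatsComponent.
; Box hit (physics) and begin-overlap (non-physics) events both forward the actor and stats to CallOnProjectileHit; only hits include hit results.
; The construction script applies the CollisionProfileName variable to the box and zeroes ProjectileMovement's initial and max speed, leaving launch speed unset here.
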(event OnComponentHit(Box)
  (params (HitComponent :type Primitive%20Component%20Object%20Reference) (OtherActor :type Actor%20Object%20Reference) (OtherComp :type Primitive%20Component%20Object%20Reference) (NormalImpulse :type Vector :default "0, 0, 0") (Hit :type Hit%20Result%20Structure%20%28by%20ref%29))
  (bind _returnvalue (Actor|GetComponentbyClass OtherActor "/Script/CombatStatsComponent.CombatStatsComponent"))
  ;[1 1 1] Hit (Physics-Based)
  (Utilities|IsValid _returnvalue
    (:Is%20Valid
      (Default|CallOnProjectileHit OtherActor Hit _returnvalue))))

(event OnComponentBeginOverlap(Box)
  (params (OverlappedComponent :type Primitive%20Component%20Object%20Reference) (OtherActor :type Actor%20Object%20Reference) (OtherComp :type Primitive%20Component%20Object%20Reference) (OtherBodyIndex :type Integer) (bFromSweep :type Boolean) (SweepResult :type Hit%20Result%20Structure%20%28by%20ref%29))
  (bind _returnvalue (Actor|GetComponentbyClass OtherActor "/Script/CombatStatsComponent.CombatStatsComponent"))
  ;[1 1 1] Overlap (No Physics)
  (Utilities|IsValid _returnvalue
    (:Is%20Valid
      (Default|CallOnProjectileHit :Other%20Actor OtherActor :Combat%20Stats _returnvalue))))

(event EventBeginPlay)

(event Collision|EventActorBeginOverlap
  (params (OtherActor :type Actor%20Object%20Reference)))

(event EventTick
  (params (DeltaSeconds :type Float%20%28single-precision%29)))

(fn ConstructionScript
  (bind _projectilemovement (Variables|Default|GetProjectileMovement))
  (Variables|/Script/Engine.ProjectileMovementComponent|SetMaxSpeed _projectilemovement 0.0)
  (Variables|/Script/Engine.ProjectileMovementComponent|SetInitialSpeed _projectilemovement 0.0)
  (Collision|SetCollisionProfileName (Variables|Default|GetBox) (Variables|ProjectileSettings|GetCollision%20Profile%20Name) true :!class /Script/Engine.PrimitiveComponent))