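; BP_Projectile_Move is a projectile Blueprint that applies a combat move's data when it hits.
; Its construction script runs the parent's, then binds an event to OnProjectileHit.
; Apply MoveData passes the ProjectileMove's MoveData to a CombatStats object's ApplyMoveData, with CombatStats also given as the attacker.
; The event graph holds only disabled placeholder events.
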(event EventBeginPlay
  (|CallParentFunction) ; This node is disabled and will not be called.\nDrag off pins to build functionality.
)

(event Collision|EventActorBeginOverlap
  (params (OtherActor :type Actor%20Object%20Reference))
  (|CallParentFunction OtherActor) ; This node is disabled and will not be called.\nDrag off pins to build functionality.
)

(event EventTick
  (params (DeltaSeconds :type Float%20%28single-precision%29))
  (|CallParentFunction DeltaSeconds) ; This node is disabled and will not be called.\nDrag off pins to build functionality.
)

(fn ConstructionScript
  (|CallParentFunction)
  (EventDispatchers|BindEventtoOnProjectileHit (EventDispatchers|CreateEvent :!event ApplyMoveData)))

(fn ApplyMoveData
  (params (Other%20Actor :type Actor%20Object%20Reference) (Hit%20Results :type Hit%20Result%20Structure) (Combat%20Stats :type Combat%20Stats%20Component%20Object%20Reference))
  (Class|CombatStatsComponent|ApplyMoveData Combat%20Stats (Variables|/Script/BattleEngine.ProjectileMove|GetMoveData (Variables|Default|GetProjectileMove)) (Variables|ExternalReferences|GetCombatStats)))