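; Healing tree move actor that applies a Regrowth effect to actors overlapping its OverlapTracker.
; An actor's first overlap casts Regrowth immediately and starts a per-actor cooldown in the CDs map.
; Tick counts cooldowns down and recasts only if the actor still overlaps at expiry.
; Entries are never removed, so an actor returning after expiry gets no further casts.
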(event BeginOverlap(OverlapTracker)
  (params (OverlappedComp :type Primitive%20Component%20Object%20Reference) (OtherActor :type Actor%20Object%20Reference) (OtherComp :type Primitive%20Component%20Object%20Reference) (OtherBodyIndex :type Integer) (bFromSweep :type Boolean) (SweepResult :type Hit%20Result%20Structure%20%28by%20ref%29))
  (CallFunction|RegisterNewCD OtherActor))

(event EventBeginPlay)

(event Collision|EventActorBeginOverlap
  (params (OtherActor :type Actor%20Object%20Reference)))

(event EventTick
  (params (DeltaSeconds :type Float%20%28single-precision%29))
  (CallFunction|UpdateCDs DeltaSeconds))

(fn ConstructionScript)

(fn UpdateCDs
  (params (Dt :type Float%20%28double-precision%29))
  (bind _keys (Utilities|Map|Keys (Variables|Default|GetCDs)))
  (for _array_element _keys
    (LocalVariables|SetCurrent%20Actor _array_element)
    (if (> (.Value (Utilities|Map|Find (Variables|Default|GetCDs) (LocalVariables|GetCurrent%20Actor))) 0.0)
      (Utilities|Map|Add (Variables|Default|GetCDs) (LocalVariables|GetCurrent%20Actor) (- (.Value (Utilities|Map|Find (Variables|Default|GetCDs) (LocalVariables|GetCurrent%20Actor))) Dt))
      (if (and (<= (- (.Value (Utilities|Map|Find (Variables|Default|GetCDs) (LocalVariables|GetCurrent%20Actor))) Dt) 0.0) (Utilities|Array|ContainsItem (Class|OverlapTracker|GetOverlappingActors (Variables|Default|GetOverlapTracker)) (LocalVariables|GetCurrent%20Actor)))
        (CallFunction|CastRegrowth (LocalVariables|GetCurrent%20Actor))))))

(fn RegisterNewCD
  (params (New%20Actor :type Actor%20Object%20Reference))
  (if (not (Utilities|Map|Contains (Variables|Default|GetCDs) New%20Actor))
    (Utilities|Map|Add (Variables|Default|GetCDs) New%20Actor 0.0)
    (CallFunction|CastRegrowth New%20Actor)))

(fn CastRegrowth
  (params (Target :type Actor%20Object%20Reference))
  (Game|AddComponentbyClass Target "/Script/HoTComponent.Regrowth")
  (Utilities|Map|Add (Variables|Default|GetCDs) Target (Variables|Default|GetEffect%20Cooldown))
  (Development|PrintString (Utilities|String|Append "Casting regrowth on " (Utilities|GetDisplayName Target))))